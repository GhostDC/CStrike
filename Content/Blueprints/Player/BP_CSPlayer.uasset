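; BP_CSPlayer is the player Blueprint that binds input to movement, look, weapon and drop actions.
; Axis events pass values to MoveForward and MoveRight, and feed Turn and LookUp straight into controller yaw and pitch.
; Pressed events for primary fire, secondary fire, reload and drop each call a matching function.
; The graph is a thin input layer: those gameplay functions are defined outside it, and the construction script is empty.
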(event `InputAxis|MoveForward`
  (params (AxisValue :type "Float (single-precision)"))
  ;[1 1 1] Movement
  (`self.MoveForward` AxisValue))

(event `InputAction|PrimaryFire`
  (params (Key :type "Key Structure"))
  (:`Pressed`
    (`self.PlayerFirePrimary`)))

(event `InputAxis|MoveRight`
  (params (AxisValue :type "Float (single-precision)"))
  ;[1 1 1] Movement
  (`self.MoveRight` AxisValue))

(event `InputAction|SecondaryFire`
  (params (Key :type "Key Structure"))
  (:`Pressed`
    (`self.PlayerFireSecondary`)))

(event `InputAxis|Turn`
  (params (AxisValue :type "Float (single-precision)"))
  ;[1 1 1] Movement
  (`self.AddControllerYawInput` AxisValue))

(event `InputAction|Reload`
  (params (Key :type "Key Structure"))
  (:`Pressed`
    (`self.PlayerReload`)))

(event `InputAxis|LookUp`
  (params (AxisValue :type "Float (single-precision)"))
  ;[1 1 1] Movement
  (`self.AddControllerPitchInput` AxisValue))

(event `InputAction|Drop`
  (params (Key :type "Key Structure"))
  (:`Pressed`
    (`self.Drop`)))

(fn `UserConstructionScript`)